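; Master weapon Blueprint for a world pickup that the player's ThirdPersonCharacter can take with the equipWeapon input.
; An overlap volume stores the character and an in-range flag and enables player input, so pressing the action calls Pickup on that character with itself.
; The construction script writes the actor's own class into its ItemInfo struct, and an offAll event destroys the collision component.
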(event OnComponentBeginOverlap(cullision)
  (params (OverlappedComponent :type Primitive%20Component%20Object%20Reference) (OtherActor :type Actor%20Object%20Reference) (OtherComp :type Primitive%20Component%20Object%20Reference) (OtherBodyIndex :type Integer) (bFromSweep :type Boolean) (SweepResult :type Hit%20Result%20Structure%20%28by%20ref%29))
  (bind _asthird_person_character (Utilities|Casting|CastToThirdPersonCharacter OtherActor))
  (Variables|Default|Setsgref _asthird_person_character)
  (Variables|Default|SetisInRange true)
  (Input|EnableInput (Game|GetPlayerController 0)))

(event OnComponentEndOverlap(cullision)
  (params (OverlappedComponent :type Primitive%20Component%20Object%20Reference) (OtherActor :type Actor%20Object%20Reference) (OtherComp :type Primitive%20Component%20Object%20Reference) (OtherBodyIndex :type Integer))
  (Utilities|Casting|CastToThirdPersonCharacter OtherActor)
  (Variables|Default|Setsgref 0)
  (Variables|Default|SetisInRange false))

(event Custom|offAll
  (Components|DestroyComponent (Variables|Default|Getcullision)))

(event Input|ActionEvents|InputActionequipWeapon
  (params (Key :type Key%20Structure :default "None"))
  (:Pressed
    (if (Variables|Default|GetisInRange)
      (Default|Pickup (Variables|Default|Getsgref) self))))

(fn ConstructionScript
  (Variables|Default|SetitemInfo (Utilities|Struct|MakeitemType (.itemtype (Variables|Default|GetitemInfo)) (Utilities|GetClass self) (.currentammo (Variables|Default|GetitemInfo)) (.maxammo (Variables|Default|GetitemInfo)) (.damage (Variables|Default|GetitemInfo)) (.itemimage (Variables|Default|GetitemInfo)) (.equipsocet (Variables|Default|GetitemInfo)) (.unequipsocet (Variables|Default|GetitemInfo)))))